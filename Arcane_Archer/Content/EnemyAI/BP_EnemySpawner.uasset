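; BP_EnemySpawner is an actor that spawns BP_EnemyAI enemies near its own location.
; SpawnEnemy picks a random horizontal offset around the spawner, projects it onto the navmesh, and spawns the enemy there with a fixed facing only if projection succeeds.
; It returns the new enemy, and nothing in this Blueprint calls it, as the event graph is empty.
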(event EventBeginPlay)

(event Collision|EventActorBeginOverlap
  (params (OtherActor :type Actor%20Object%20Reference)))

(event EventTick
  (params (DeltaSeconds :type Float%20%28single-precision%29)))

(fn ConstructionScript)

(fn SpawnEnemy
  (bind _output_get (Variables|Default|SetActorLocation (Transformation|GetActorLocation)))
  (bind _output_get_2 (Variables|Default|SetSpawnLocation (+ _output_get (Math|Vector|MakeVector (Math|Random|RandomFloatinRange -3e+02 3e+02) (Math|Random|RandomFloatinRange -3e+02 3e+02) 0.0))))
  (if (.ReturnValue (AI|Navigation|ProjectPointtoNavigation _output_get_2 0 0 "0, 0, 0"))
    (bind _returnvalue (Game|SpawnActorfromClass "/Game/EnemyAI/BP_EnemyAI.BP_EnemyAI_C" (Math|Transform|MakeTransform (.ProjectedLocation (AI|Navigation|ProjectPointtoNavigation _output_get_2 0 0 "0, 0, 0")) (Math|Rotator|MakeRotator 0.0 0.0 1.8e+02)) "Undefined" "MultiplyWithRoot" 0 0))
    (return _returnvalue)))