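; Enemy AI character that chases the player once a BP_FirstPersonCharacter enters its AggroRange.
; The overlap latches IsPlayerDetected, and Tick then issues AIMoveTo toward the player's current location, with nothing here clearing the flag.
; BeginPlay adds an enemy attack component, and UpdateWalkSpeed sets max walk speed.
; PawnSensing and FollowPlayer events are empty, and an alternative sight-based chase is left disconnected.
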(event OnSeePawn(PawnSensing)
  (params (Pawn :type Pawn%20Object%20Reference)))

(event OnComponentBeginOverlap(AggroRange)
  (params (OverlappedComponent :type Primitive%20Component%20Object%20Reference) (OtherActor :type Actor%20Object%20Reference) (OtherComp :type Primitive%20Component%20Object%20Reference) (OtherBodyIndex :type Integer) (bFromSweep :type Boolean) (SweepResult :type Hit%20Result%20Structure%20%28by%20ref%29))
  (Utilities|Casting|CastToBP_FirstPersonCharacter OtherActor)
  (Variables|Default|SetIsPlayerDetected true))

(event Custom|FollowPlayer)

(event EventBeginPlay
  (AddComponent|AddEnemyAttackComponent))

(event Collision|EventActorBeginOverlap
  (params (OtherActor :type Actor%20Object%20Reference)))

(event EventTick
  (params (DeltaSeconds :type Float%20%28single-precision%29))
  (if (Variables|Default|GetIsPlayerDetected)
    (AI|AIMoveTo self (Transformation|GetActorLocation (Game|GetPlayerCharacter 0)) 0 5.0 false)))

(fn ConstructionScript)

(fn UpdateWalkSpeed
  (params (NewWalkSpeed :type Float%20%28double-precision%29))
  (Variables|/Script/Engine.CharacterMovementComponent|SetMaxWalkSpeed (Variables|Character|GetCharacterMovement) NewWalkSpeed))